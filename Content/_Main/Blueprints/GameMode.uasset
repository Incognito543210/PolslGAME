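; Game mode that runs a wave-based enemy survival match, from the first wave through to the win screen.
; Each wave spawns zombies, knights and goats at fixed transforms, scaled by wave number, plus an ammo crate on FieldMap.
; EnemyKilled counts down the remaining enemies; a cleared wave levels up the player and shows wave UI before a delayed spawn.
; Clearing the final wave shows the player's win UI.
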(event Custom|StartGame
  ;[1 1 1] Start Game
  (bind _returnvalue (Actor|GetActorOfClass "/Game/_Main/Blueprints/BP_FirstPersonCharacter.BP_FirstPersonCharacter_C"))
  (Variables|Default|SetFirst%20Person%20Ref _returnvalue)
  (CallFunction|SpawnEnemies))

(event Custom|SpawnEnemies
  ;[1 1 1] Spawn Enemies
  (CallFunction|SpawnAmmo)
  (bind _output_get (Variables|Default|SetZombieTotal (* (Variables|Default|GetCurrentWave) 4)))
  (Variables|Default|SetZombiesLeft _output_get)
  (bind _index (Utilities|FlowControl|ForLoopwithBreak 0 _output_get :!label _label)
    (:LoopBody
      (if (== _index (/ (Variables|Default|GetZombieTotal) 4))
        (goto _label Break)
        (else
          (Game|SpawnActorfromClass "/Game/_Main/Enemies/Zombie/BP_Zombie.BP_Zombie_C" (Variables|Default|GetSpawn%20Location1) "Undefined" "MultiplyWithRoot" 0 0)
          (Game|SpawnActorfromClass "/Game/_Main/Enemies/Knight/BP_Knight.BP_Knight_C" (Variables|Default|GetSpawn%20Location6) "Undefined" "MultiplyWithRoot" 0 0))))
    (:Completed
      (Utilities|FlowControl|ForLoopwithBreak 1 (/ (Variables|Default|GetZombieTotal) 4)
        (:LoopBody
          (Game|SpawnActorfromClass "/Game/_Main/Enemies/Goat/BP_Goat.BP_Goat_C" (Variables|Default|GetSpawn%20Location3) "Undefined" "MultiplyWithRoot" 0 0)
          (Game|SpawnActorfromClass "/Game/_Main/Enemies/Zombie/BP_Zombie.BP_Zombie_C" (Variables|Default|GetSpawn%20Location2) "Undefined" "MultiplyWithRoot" 0 0))))))

(event Custom|EnemyKilled
  ;[1 1 1] Enemy Killed
  (bind _result (Math|Integer|DecrementInt (Variables|Default|GetZombiesLeft))
    (:%20%20
      (if (== _result 0)
        (CallFunction|WaveIncrement)))))

(event Custom|WaveIncrement
  ;[1 1 1] Wave Incriment
  (if (== (Variables|Default|GetCurrentWave) (Variables|Default|GetMaxWaves))
    (CallFunction|PlayerWins)
    (else
      (Math|Integer|IncrementInt (Variables|Default|GetCurrentWave)
        (:%20%20
          (Default|LevelUpCharacter (Variables|Default|GetFirst%20Person%20Ref))
          (CallFunction|WaveStart))))))

(event Custom|SpawnAmmo
  ;[1 1 1] Spawn Ammo Crate
  (bind _returnvalue (Game|GetCurrentLevelName true))
  (if (Utilities|Enum|Equal(Enum) _returnvalue "FieldMap")
    (Game|SpawnActorfromClass "/Game/_Main/Blueprints/BP_AmmoPickUp.BP_AmmoPickUp_C" (Math|Transform|MakeTransform (Utilities|Array|Get(acopy) (Variables|Default|GetAmmoCrateLocation)) "0, 0, 0" "1.000000,1.000000,1.000000") "Undefined" "MultiplyWithRoot" 0 0)))

(event Custom|WaveStart
  ;[1 1 1] Start Next Wave
  (bind _asbp_first_person_character (Utilities|Casting|CastToBP_FirstPersonCharacter (Game|GetPlayerCharacter 0)))
  (Default|ShowWaveUI _asbp_first_person_character (Variables|Default|GetCurrentWave))
  (Utilities|FlowControl|Delay 5.0)
  (CallFunction|SpawnEnemies))

(event Custom|Player%20Wins
  ;[1 1 1] Win Logic
  (bind _asbp_first_person_character (Utilities|Casting|CastToBP_FirstPersonCharacter (Game|GetPlayerCharacter 0)))
  (Default|ShowWinUI _asbp_first_person_character))

(event EventBeginPlay
  ;[1 1 1] Start Game
  (CallFunction|StartGame))

(fn ConstructionScript)